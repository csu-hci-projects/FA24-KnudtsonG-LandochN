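; Ammo pickup that bobs in place and gives the first-person character ammo on overlap.
; On BeginPlay it stores its origin, then a timeline offsets the actor from that point, with a FlipFlop on Finished alternating play and reverse to loop the motion.
; Overlap with BP_FirstPersonCharacter adds Amount to the character's Ammo and destroys the pickup.
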(event `self.ReceiveBeginPlay`
  (bind _output_get (set `self.origin` (`self.K2_GetActorLocation`)))
  (`/Engine/EditorBlueprintResources/StandardMacros.FlipFlop` :!label _label
    (:`A`
      (bind (_direction _location) (`Timeline|Timeline` :!label _label_2)
        (:`Update`
          (`self.K2_SetActorLocation` (+ _location _output_get)))
        (:`Finished`
          (goto _label))))
    (:`B`
      (goto _label_2 :!via `Reverse`))))

(event `self.ReceiveActorBeginOverlap`
  (params (OtherActor :type "Actor Object Reference"))
  (bind _asbp_first_person_character (cast `/Game/FirstPerson/Blueprints/BP_FirstPersonCharacter` OtherActor))
  (set `/Game/FirstPerson/Blueprints/BP_FirstPersonCharacter.Ammo` (+ (`/Game/FirstPerson/Blueprints/BP_FirstPersonCharacter.Ammo` _asbp_first_person_character) (`self.amount`)) _asbp_first_person_character)
  (`self.K2_DestroyActor`))

(fn `UserConstructionScript`)