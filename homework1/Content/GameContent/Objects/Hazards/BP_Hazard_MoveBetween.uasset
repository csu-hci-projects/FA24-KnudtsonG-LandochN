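; Moving hazard actor that shuttles between two points and changes the player's health on overlap.
; On BeginPlay it stores its origin and sets the timeline rate from Time, then offsets its location by the timeline curve scaled by MovementScale.
; A FlipFlop re-triggered on timeline finish alternates play and reverse for continuous motion.
; Overlapping BP_FirstPersonCharacter applies HealthChange and prints the resulting health.
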(event `self.ReceiveActorBeginOverlap`
  (params (OtherActor :type "Actor Object Reference"))
  ;[0 0 0] Damages player on collision
  ;;[1 1 1] On overlap, check if overlapping object is player
  (bind _asbp_first_person_character (cast `/Game/FirstPerson/Blueprints/BP_FirstPersonCharacter` OtherActor))
  ;;[1 1 1] If player, change health
  (`/Game/FirstPerson/Blueprints/BP_FirstPersonCharacter.ChangeHealth` _asbp_first_person_character (`self.HealthChange`))
  (`KismetSystemLibrary.PrintString` (`KismetStringLibrary.Conv_IntToString` (`/Game/FirstPerson/Blueprints/BP_FirstPersonCharacter.Health` _asbp_first_person_character))))

(event `self.ReceiveBeginPlay`
  ;[0 0 0] Moves object between two points
  ;;[1 1 1] Storing of origin point, conversion of movement time into movement rate
  (bind _output_get (set `self.Origin` (`self.K2_GetActorLocation`)))
  (`TimelineComponent.SetPlayRate` (`self.Timeline`) (/ 1.0 (`self.Time`)))
  ;;[1 1 1] Movement
  (`/Engine/EditorBlueprintResources/StandardMacros.FlipFlop` :!label _label
    (:`A`
      (bind (_direction _x_location) (`Timeline|Timeline` :!label _label_2)
        (:`Update`
          (`self.K2_SetActorLocation` (+ (* _x_location (`self.Movement scale`)) _output_get)))
        (:`Finished`
          (goto _label))))
    (:`B`
      (goto _label_2 :!via `Reverse`))))

(fn `UserConstructionScript`)